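; Jing Yuan NPC Blueprint that runs a branching dialogue with the player and shows an interaction prompt in range.
; Talk steps through lines loaded from a data table into the player's DialogueUI, pausing for choices, which jump by index.
; StartTalk and FinishTalk toggle the interface and animation Blueprint state.
; Overlapping Collision1 starts a ten-second timer for a hidden two-line exchange with Lumine, whose flag is never cleared.
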(event `/Game/Assets/UI/Dialogue/BPI_Dialogue.Talk`
  (params (index :type Integer))
  ;[1 1 1] start talk and loop until wait for choice
  (if (not (`self.InHiddenEvent`))
    (`|ExecutionSequence`
      (:`then_0`
        ;;[1 1 1] set index
        ;; if choice made(event trigger by click choice button, input index is set to index of next sentence), set index
        ;; else(event trigger by press F, input index is set to -1), increase index to goto next sentence
        (if (== index -1)
          (`/Engine/EditorBlueprintResources/StandardMacros.IncrementInt` (`self.talkIndex`)
            (:`  `
              _))
          (else
            (set `self.talkIndex` index)
            (set `self.isInChoice` false)))
        ;;[1 1 1] if not in dialogue, show interface
        (if (not (`self.isInDialogue`))
          (`self.startTalk`)))
      (:`then_1`
        ;;[1 1 1] if waiting choice, do nothing
        (if (not (`self.isInChoice`))
          ;;[1 1 1] if it's end, finish talk
          (if (`self.isEnd`)
            (`self.finishTalk`)
            (else
              ;;[1 1 1] get sentence and show, check if next is choice or end
              (bind (_haschoice _isend) (`/Game/Assets/UI/Dialogue/WBP_Dialogue.Show Dialogue` (`self.Dialogue UI`) (`self.name`) (`|GetArrayItem` (`self.dialogue`) (`self.talkIndex`))))
              (set `self.isInChoice` _haschoice)
              (set `self.isEnd` _isend))))))
    (else
      ;;[1 1 1] check if in the hidden event
      (if (`self.isEnd`)
        (`self.finishTalk`)
        (else
          (bind _returnvalue (`|GetDataTableRow` "/Game/Assets/Data/Dialogue/JingYuan_hidden_event.JingYuan_hidden_event" "1")
            (:`then`
              (`/Game/Assets/UI/Dialogue/WBP_Dialogue.Show Dialogue` (`self.Dialogue UI`) "Lumine" _returnvalue)
              (set `self.isEnd` true))))))))

(event `self.ReceiveBeginPlay`
  ;[1 1 1] get UI and dialogue text
  (`|ExecutionSequence`
    (:`then_0`
      (`KismetSystemLibrary.Delay` 5.0)
      (bind _asplayer_bp (cast `/Game/Assets/Charactor_model/Lumine/BP/Player_BP` (`GameplayStatics.GetPlayerCharacter` 0)))
      (set `self.player` _asplayer_bp)
      (set `self.Prompt UI` (`/Game/Assets/Charactor_model/Lumine/BP/Player_BP.PromptUI` _asplayer_bp))
      (set `self.Dialogue UI` (`/Game/Assets/Charactor_model/Lumine/BP/Player_BP.DialogueUI` _asplayer_bp)))
    (:`then_1`
      (bind _outrownames (`DataTableFunctionLibrary.GetDataTableRowNames` "/Game/Assets/Data/Dialogue/JingYuan_dialogue_table.JingYuan_dialogue_table"))
      (for _array_element _outrownames
        (bind _returnvalue (`|GetDataTableRow` "/Game/Assets/Data/Dialogue/JingYuan_dialogue_table.JingYuan_dialogue_table" _array_element)
          (:`then`
            (`KismetArrayLibrary.Array_Add` (`self.dialogue`) _returnvalue)))))))

(event `self.Interact_range.OnComponentBeginOverlap`
  (params (OverlappedComponent :type "PrimitiveComponent Object Reference") (OtherActor :type "Actor Object Reference") (OtherComp :type "PrimitiveComponent Object Reference") (OtherBodyIndex :type Integer) (bFromSweep :type Boolean) (SweepResult :type "HitResult Structure (by ref)"))
  (bind _prompt_ui (`self.Prompt UI`))
  ;[1 1 1] prompt
  (if (== OtherActor (`GameplayStatics.GetPlayerCharacter` 0))
    (`UserWidget.AddToViewport` _prompt_ui 0)
    (`TextBlock.SetText` (`/Game/Assets/UI/Dialogue/WBP_prompt.name` _prompt_ui) (`self.name`))))

(event `self.Interact_range.OnComponentEndOverlap`
  (params (OverlappedComponent :type "PrimitiveComponent Object Reference") (OtherActor :type "Actor Object Reference") (OtherComp :type "PrimitiveComponent Object Reference") (OtherBodyIndex :type Integer))
  ;[1 1 1] prompt
  (if (== (`GameplayStatics.GetPlayerCharacter` 0) OtherActor)
    (`Widget.RemoveFromParent` (`self.Prompt UI`))))

(event `self.collision1.OnComponentBeginOverlap`
  (params (OverlappedComponent :type "PrimitiveComponent Object Reference") (OtherActor :type "Actor Object Reference") (OtherComp :type "PrimitiveComponent Object Reference") (OtherBodyIndex :type Integer) (bFromSweep :type Boolean) (SweepResult :type "HitResult Structure (by ref)"))
  ;[1 1 1] hidden event
  (`KismetSystemLibrary.K2_SetTimerDelegate` (delegate `hiddenEvent`) 10.0))

(event `self.collision1.OnComponentEndOverlap`
  (params (OverlappedComponent :type "PrimitiveComponent Object Reference") (OtherActor :type "Actor Object Reference") (OtherComp :type "PrimitiveComponent Object Reference") (OtherBodyIndex :type Integer))
  ;[1 1 1] hidden event
  (`KismetSystemLibrary.K2_ClearTimer` null "hiddenEvent"))

(event `hiddenEvent`
  ;[1 1 1] hidden event
  (set `self.InHiddenEvent` true)
  (`self.startTalk`)
  (bind _returnvalue (`|GetDataTableRow` "/Game/Assets/Data/Dialogue/JingYuan_hidden_event.JingYuan_hidden_event" "0")
    (:`then`
      (`/Game/Assets/UI/Dialogue/WBP_Dialogue.Show Dialogue` (`self.Dialogue UI`) "Jing Yuan" _returnvalue))))

(fn `finishTalk`
  (`|ExecutionSequence`
    (:`then_0`
      ;[1 1 1] remove interface
      (`/Game/Assets/Charactor_model/Lumine/BP/Player_BP.InterfacesOpen&Close` :`self` (`self.player`) :`interface` "NewEnumerator5"))
    (:`then_1`
      ;[1 1 1] set npc animation to idle
      (bind _asjing_yuan_anim (cast `/Game/Assets/Charactor_model/JingYuan/BP/JingYuan_Anim` (`SkeletalMeshComponent.GetAnimInstance` (`self.model`))))
      (set `/Game/Assets/Charactor_model/JingYuan/BP/JingYuan_Anim.IsInDialogue` false _asjing_yuan_anim))
    (:`then_2`
      ;[1 1 1] set state
      (set `self.isInDialogue` false))))

(fn `startTalk`
  (`|ExecutionSequence`
    (:`then_0`
      ;[1 1 1] set IsInDialogue to true in animation blueprint
      (bind _asjing_yuan_anim (cast `/Game/Assets/Charactor_model/JingYuan/BP/JingYuan_Anim` (`SkeletalMeshComponent.GetAnimInstance` (`self.model`))))
      (set `/Game/Assets/Charactor_model/JingYuan/BP/JingYuan_Anim.IsInDialogue` true _asjing_yuan_anim))
    (:`then_1`
      ;[1 1 1] set param
      (set `self.isInDialogue` true)
      (set `self.isEnd` false)
      (set `self.isInChoice` false)
      (set `self.talkIndex` 0))
    (:`then_2`
      ;[1 1 1] show interface
      (`/Game/Assets/Charactor_model/Lumine/BP/Player_BP.InterfacesOpen&Close` :`self` (`self.player`) :`open` true :`interface` "NewEnumerator5"))))

(fn `UserConstructionScript`)