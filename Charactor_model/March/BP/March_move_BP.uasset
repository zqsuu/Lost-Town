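; Scripted scene actor that moves March along a spline, then stages a dialogue with March, Dan Heng and the player.
; A timeline curve scaled by spline length drives March's location and rotation; on finish March switches to idle and all three characters snap to fixed spots.
; Talk steps through indexed lines, waits for a valid choice at one step, then closes the UI and teleports the player away.
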(event `self.ReceiveBeginPlay`)

(event `move`
  (bind _spline (`self.Spline`))
  (bind _march (`self.March`))
  (bind _talkindex (`self.talkIndex`))
  (bind (_direction _curve) (`Timeline|时间轴` :!via `PlayFromStart`)
    (:`Update`
      (bind _returnvalue (* _curve (`SplineComponent.GetSplineLength` _spline)))
      (`self.K2_SetActorLocationAndRotation` _march (`SplineComponent.GetLocationAtDistanceAlongSpline` _spline _returnvalue "World") (`SplineComponent.GetRotationAtDistanceAlongSpline` _spline _returnvalue "World") false false))
    (:`Finished`
      (`|ExecutionSequence`
        (:`then_0`
          ;[1 1 1] march
          (bind _asmarch_char_bp (cast `/Game/Assets/Charactor_model/March/BP/March_char_BP` _march))
          (`SkeletalMeshComponent.SetAnimation` (`/Game/Assets/Charactor_model/March/BP/March_char_BP.March` _asmarch_char_bp) "/Game/Assets/Charactor_model/March/BP/March_idle.March_idle")
          (`self.K2_SetActorLocationAndRotation` _march (-2220.0 -1690.0 1815.0) (struct :`Yaw` -100.0) false false))
        (:`then_1`
          ;[1 1 1] Dan Heng
          (`self.K2_SetActorLocationAndRotation` (`self.Dan heng`) (-2380.0 -1730.0 1815.0) (struct :`Yaw` -100.0) false false))
        (:`then_2`
          ;[1 1 1] set player location
          (bind _asplayer_bp (cast `/Game/Assets/Charactor_model/Lumine/BP/Player_BP` (`GameplayStatics.GetPlayerCharacter` 0)))
          (bind _output_get (set `self.player` _asplayer_bp))
          (`self.K2_SetActorLocationAndRotation` _output_get (-2170.0 -1830.0 1815.0) (struct :`Yaw` 140.0) false false))
        (:`then_3`
          ;[1 1 1] talk1
          (`/Game/Assets/Charactor_model/Lumine/BP/Player_BP.InterfacesOpen&Close` :`self` _asplayer_bp :`open` true :`interface` "NewEnumerator5")
          (`/Game/Assets/UI/Dialogue/WBP_Dialogue.Show Dialogue` (`/Game/Assets/Charactor_model/Lumine/BP/Player_BP.DialogueUI` _asplayer_bp) (`|GetArrayItem` (`self.name`) _talkindex) (`|GetArrayItem` (`self.dialogue`) _talkindex) :!label _label)
          (`/Engine/EditorBlueprintResources/StandardMacros.IncrementInt` _talkindex))))))

(event `/Game/Assets/UI/Dialogue/BPI_Dialogue.Talk`
  (params (index :type Integer))
  (bind _talkindex (`self.talkIndex`))
  ;[1 1 1] talk1
  (if (== _talkindex 4)
    (`/Game/Assets/Charactor_model/Lumine/BP/Player_BP.InterfacesOpen&Close` :`self` (stale `move` _asplayer_bp) :`interface` "NewEnumerator5")
    (`/Game/Assets/Charactor_model/Lumine/BP/Player_BP.InterfacesOpen&Close` :`self` (stale `move` _asplayer_bp) :`interface` "NewEnumerator6")
    (`self.K2_SetActorLocationAndRotation` (`self.player`) (-10090.0 -860.0 1815.0) (struct :`Yaw` 90.0) false false)
    (elif (== _talkindex 3)
      (if (!= index -1)
        (goto _label))
      (else
        (goto _label)))))

(fn `UserConstructionScript`)