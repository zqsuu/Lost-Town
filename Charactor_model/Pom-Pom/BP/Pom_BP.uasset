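; Pom-Pom NPC trigger that intercepts the player with a warning when they enter its box.
; On overlap it reveals the model, plays a black screen and teleports the player to an offset from Pom-Pom.
; It then shows a warning through Player_BP's dialogue UI, closes it after a short delay and removes the prompt.
; A second black screen, from the AnimUI widget created at BeginPlay, covers hiding the model again.
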(event `self.ReceiveBeginPlay`
  (bind _returnvalue (`|CreateWidget` "/Game/Assets/Animation/AnimUI.AnimUI_C"))
  (set `self.blackAnim` _returnvalue))

(event `self.Box.OnComponentBeginOverlap`
  (params (OverlappedComponent :type "PrimitiveComponent Object Reference") (OtherActor :type "Actor Object Reference") (OtherComp :type "PrimitiveComponent Object Reference") (OtherBodyIndex :type Integer) (bFromSweep :type Boolean) (SweepResult :type "HitResult Structure (by ref)"))
  (bind _returnvalue (`GameplayStatics.GetPlayerCharacter` 0))
  (bind _blackanim (`self.blackAnim`))
  (bind _model (`self.Model`))
  (bind _blackanim_2 (`self.blackAnim`))
  (if (== OtherActor _returnvalue)
    (`|ExecutionSequence`
      (:`then_0`
        (`SceneComponent.SetVisibility` _model true false)
        (`UserWidget.AddToViewport` _blackanim_2 0)
        (`/Game/Assets/Animation/AnimUI.playBlackScreen` _blackanim_2 1.0)
        (`self.K2_SetActorLocationAndRotation` _returnvalue (+ (`SceneComponent.GetSocketLocation` _model "None") (100.0 0.0 100.0)) (`KismetMathLibrary.MakeRotator` 0.0 0.0 180.0) false false))
      (:`then_1`
        (bind _asplayer_bp (cast `/Game/Assets/Charactor_model/Lumine/BP/Player_BP` _returnvalue))
        (`/Game/Assets/Charactor_model/Lumine/BP/Player_BP.InterfacesOpen&Close` :`self` _asplayer_bp :`open` true :`interface` "NewEnumerator5")
        (`/Game/Assets/UI/Dialogue/WBP_Dialogue.Show Dialogue` (`/Game/Assets/Charactor_model/Lumine/BP/Player_BP.DialogueUI` _asplayer_bp) "Pom-Pom" (make `/Game/Assets/Data/Dialogue/dialogue_struct` "Hey you! Don't do this, it's too dangerous!" "" 0 "" 0 true))
        (`KismetSystemLibrary.Delay` 3.0)
        (`/Game/Assets/Charactor_model/Lumine/BP/Player_BP.InterfacesOpen&Close` :`self` _asplayer_bp :`interface` "NewEnumerator5")
        (`Widget.RemoveFromParent` (`/Game/Assets/Charactor_model/Lumine/BP/Player_BP.PromptUI` _asplayer_bp))
        (`|ExecutionSequence`
          (:`then_0`
            (`UserWidget.AddToViewport` _blackanim 0)
            (`/Game/Assets/Animation/AnimUI.playBlackScreen` _blackanim 1.0))
          (:`then_1`
            (`KismetSystemLibrary.Delay` 0.4)
            (`SceneComponent.SetVisibility` (`self.Model`) false false)))))))

(fn `UserConstructionScript`)