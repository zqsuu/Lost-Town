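; Kaveh NPC Blueprint that shows an interact prompt in range and runs a branching dialogue offering a transaction interface and a house upgrade.
; Talk steps through lines loaded from a DataTable, pausing at choices and jumping to the selected index.
; Hard-coded indices open the transaction UI or spend money and wood to play the upgrade sequence once.
; FinishTalk resets the animation dialogue flag, but StartTalk's code setting it is unconnected.
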(event `self.Talk`
  (params (index :type Integer))
  (bind _talkindex (`self.talkIndex`))
  (bind _items (`/Game/Assets/Charactor_model/Lumine/BP/Player_BP.items` (`self.player`)))
  ;[1 1 1] start talk and loop until wait for choice
  (`|ExecutionSequence`
    (:`then_0`
      ;;[1 1 1] set index
      ;; if choice made(event trigger by click choice button, input index is set to index of next sentence), set index
      ;; else(event trigger by press F, input index is set to -1), increase index to goto next sentence
      (if (== index -1)
        (`/Engine/EditorBlueprintResources/StandardMacros.IncrementInt` (`self.talkIndex`)
          (:`  `
            _))
        (else
          (set `self.talkIndex` index)
          (set `self.isInChoice` false)))
      ;;[1 1 1] if not in dialogue, show interface
      (if (not (`self.isInDialogue`))
        (`self.startTalk`)))
    (:`then_1`
      ;;[1 1 1] if waiting choice, do nothing
      (if (`self.isInChoice`)
        _
        (elif (`self.isEnd`)
          ;;[1 1 1] if it's end, finish talk
          (`self.finishTalk`)
          (elif (== _talkindex 4)
            (`self.finishTalk`)
            ;[0 0.8899 1] open transaction interface
            (`/Game/Assets/Charactor_model/Lumine/BP/Player_BP.InterfacesOpen&Close` (`self.player`) true "NewEnumerator1" (`self.class`))
            (elif (== _talkindex 3)
              (if (`self.isUpgraded?`)
                ;[1 1 1] upgrade house
                (bind (_haschoice _isend) (`/Game/Assets/UI/Dialogue/WBP_Dialogue.Show Dialogue` (`self.Dialogue UI`) (`self.name`) (make `/Game/Assets/Data/Dialogue/dialogue_struct` "You have upgraded your house." "" 0 "" 0 true)))
                (set `self.isInChoice` _haschoice)
                (set `self.isEnd` _isend)
                (elif (and (>= (`/Game/Assets/Data/Items/AC_Items.money` _items) 1000) (>= (`BlueprintMapLibrary.Map_Find` (`/Game/Assets/Data/Items/AC_Items.backpack` _items) "wood") 100))
                  (`/Game/Assets/Data/Items/AC_Items.change_money` _items -1000)
                  (`/Game/Assets/Data/Items/AC_Items.change_backpack` _items "wood" -100)
                  (set `self.isUpgraded?` true)
                  (bind (_outactor _returnvalue) (`LevelSequencePlayer.CreateLevelSequencePlayer` "/Game/Assets/Animation/UpgradeHouse.UpgradeHouse"))
                  (`MovieSceneSequencePlayer.Play` _returnvalue)
                  (`self.finishTalk`)
                  (else
                    (bind (_haschoice_2 _isend_2) (`/Game/Assets/UI/Dialogue/WBP_Dialogue.Show Dialogue` (`self.Dialogue UI`) (`self.name`) (make `/Game/Assets/Data/Dialogue/dialogue_struct` "You don't have enough supplies." "" 0 "" 0 true)))
                    (set `self.isInChoice` _haschoice_2)
                    (set `self.isEnd` _isend_2))))
              (else
                ;;[1 1 1] get sentence and show, check if next is choice or end
                (bind (_haschoice_3 _isend_3) (`/Game/Assets/UI/Dialogue/WBP_Dialogue.Show Dialogue` (`self.Dialogue UI`) (`self.name`) (`|GetArrayItem` (`self.dialogue`) (`self.talkIndex`))))
                (set `self.isInChoice` _haschoice_3)
                (set `self.isEnd` _isend_3)))))))))

(event `self.ReceiveBeginPlay`
  ;[1 1 1] get UI and dialogue text
  (`|ExecutionSequence`
    (:`then_0`
      (`KismetSystemLibrary.Delay` 5.0)
      (bind _asplayer_bp (cast `/Game/Assets/Charactor_model/Lumine/BP/Player_BP` (`GameplayStatics.GetPlayerCharacter` 0)))
      (set `self.player` _asplayer_bp)
      (set `self.Prompt UI` (`/Game/Assets/Charactor_model/Lumine/BP/Player_BP.PromptUI` _asplayer_bp))
      (set `self.Dialogue UI` (`/Game/Assets/Charactor_model/Lumine/BP/Player_BP.DialogueUI` _asplayer_bp)))
    (:`then_1`
      ;;[0.1587 0.7472 1] set npc dialogue
      (bind _outrownames (`DataTableFunctionLibrary.GetDataTableRowNames` "/Game/Assets/Data/Dialogue/Kaveh_dialogue_table.Kaveh_dialogue_table"))
      (for _array_element _outrownames
        (bind _returnvalue (`|GetDataTableRow` "/Game/Assets/Data/Dialogue/Kaveh_dialogue_table.Kaveh_dialogue_table" _array_element)
          (:`then`
            (`KismetArrayLibrary.Array_Add` (`self.dialogue`) _returnvalue)))))))

(event `self.Interact_range.OnComponentBeginOverlap`
  (params (OverlappedComponent :type "PrimitiveComponent Object Reference") (OtherActor :type "Actor Object Reference") (OtherComp :type "PrimitiveComponent Object Reference") (OtherBodyIndex :type Integer) (bFromSweep :type Boolean) (SweepResult :type "HitResult Structure (by ref)"))
  (bind _prompt_ui (`self.Prompt UI`))
  ;[1 1 1] prompt
  (if (== OtherActor (`GameplayStatics.GetPlayerCharacter` 0))
    (`UserWidget.AddToViewport` _prompt_ui 0)
    (`TextBlock.SetText` (`/Game/Assets/UI/Dialogue/WBP_prompt.name` _prompt_ui) (`self.name`))))

(event `self.Interact_range.OnComponentEndOverlap`
  (params (OverlappedComponent :type "PrimitiveComponent Object Reference") (OtherActor :type "Actor Object Reference") (OtherComp :type "PrimitiveComponent Object Reference") (OtherBodyIndex :type Integer))
  ;[1 1 1] prompt
  (if (== (`GameplayStatics.GetPlayerCharacter` 0) OtherActor)
    (`Widget.RemoveFromParent` (`self.Prompt UI`))))

(fn `finishTalk`
  (`|ExecutionSequence`
    (:`then_0`
      ;[1 1 1] remove interface
      (`/Game/Assets/Charactor_model/Lumine/BP/Player_BP.InterfacesOpen&Close` :`self` (`self.player`) :`interface` "NewEnumerator5"))
    (:`then_1`
      ;[1 1 1] set npc animation to idle
      (bind _asjing_yuan_anim (cast `/Game/Assets/Charactor_model/JingYuan/BP/JingYuan_Anim` (`SkeletalMeshComponent.GetAnimInstance` (`self.Model`))))
      (set `/Game/Assets/Charactor_model/JingYuan/BP/JingYuan_Anim.IsInDialogue` false _asjing_yuan_anim))
    (:`then_2`
      ;[1 1 1] set state
      (set `self.isInDialogue` false))))

(fn `startTalk`
  (`|ExecutionSequence`
    (:`then_1`
      ;[1 1 1] set param
      (set `self.isInDialogue` true)
      (set `self.isEnd` false)
      (set `self.isInChoice` false)
      (set `self.talkIndex` 0))
    (:`then_2`
      ;[1 1 1] show interface
      (`/Game/Assets/Charactor_model/Lumine/BP/Player_BP.InterfacesOpen&Close` :`self` (`self.player`) :`open` true :`interface` "NewEnumerator5"))))

(fn `UserConstructionScript`)