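; AC_Items is an item component that tracks the money, backpack contents and store stock.
; On BeginPlay it reads every row of Item_Table, taking Money from the "money" row and filling the Backpack and Store maps from the others' Count and Store fields, keyed by the row's Name field.
; Three functions update that state by adding to a backpack count, adding to money or subtracting from store stock, with no bounds checks.
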(event `self.ReceiveBeginPlay`
  (bind _outrownames (`DataTableFunctionLibrary.GetDataTableRowNames` "/Game/Assets/Data/Items/Item_Table.Item_Table"))
  (for _array_element _outrownames
    (if (== _array_element "money")
      ;[1 1 1] set money
      (bind _returnvalue (`|GetDataTableRow` "/Game/Assets/Data/Items/Item_Table.Item_Table" "money")
        (:`then`
          (set `self.money` (`.count_8_2D7831E34F092340A7D6BEB6D11E65F3` (break `/Game/Assets/Data/Items/Item_Struct` _returnvalue)))))
      (else
        ;[1 1 1] set backpack
        (bind _returnvalue_2 (`|GetDataTableRow` "/Game/Assets/Data/Items/Item_Table.Item_Table" _array_element)
          (:`then`
            (bind ((`name_2_EEF2DE294D90549A2F44F59EE3817EB2` _name) (`count_8_2D7831E34F092340A7D6BEB6D11E65F3` _count)) (break `/Game/Assets/Data/Items/Item_Struct` _returnvalue_2))
            (`BlueprintMapLibrary.Map_Add` (`self.backpack`) (`KismetStringLibrary.Conv_StringToName` _name) _count)
            ;[1 1 1] set store
            (bind _returnvalue_3 (`|GetDataTableRow` "/Game/Assets/Data/Items/Item_Table.Item_Table" _array_element)
              (:`then`
                (bind ((`name_2_EEF2DE294D90549A2F44F59EE3817EB2` _name_2) (`store_29_3168FD714AB25772492E5AA2A2101A0C` _store)) (break `/Game/Assets/Data/Items/Item_Struct` _returnvalue_3))
                (`BlueprintMapLibrary.Map_Add` (`self.store`) (`KismetStringLibrary.Conv_StringToName` _name_2) _store)))))))))

(fn `change_backpack`
  (params (name :type Name) (count :type Integer))
  (bind _backpack (`self.backpack`))
  (`BlueprintMapLibrary.Map_Add` _backpack name (+ count (`BlueprintMapLibrary.Map_Find` _backpack name))))

(fn `change_money`
  (params (count :type Integer))
  (set `self.money` (+ (`self.money`) count)))

(fn `remove_store`
  (params (name :type Name) (count :type Integer))
  (bind _store (`self.store`))
  (`BlueprintMapLibrary.Map_Add` _store name (- (`BlueprintMapLibrary.Map_Find` _store name) count)))